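; Player character Blueprint that runs the opening intro and tutorial screens and handles talking to NPCs.
; BeginPlay starts music and the first intro widget; Enter advances through intro text and tutorial via boolean flags, then marks the dialogue component in-game.
; The Interact overlap caches an NPC and its BPI_Interact component and shows a prompt.
; IA_Interact starts that interaction or a come-later message, depending on IsTalkable.
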(event OnComponentBeginOverlap(Interact)
  (params (OverlappedComponent :type Primitive%20Component%20Object%20Reference) (OtherActor :type Actor%20Object%20Reference) (OtherComp :type Primitive%20Component%20Object%20Reference) (OtherBodyIndex :type Integer) (bFromSweep :type Boolean) (SweepResult :type Hit%20Result%20Structure%20%28by%20ref%29))
  (bind _asbp_base_npc (Utilities|Casting|CastToBP_BaseNPC OtherActor))
  (Variables|Default|SetNPC _asbp_base_npc)
  (Variables|Default|SetDialogueActor (Utilities|Array|Get(acopy) (Class|Actor|GetComponentsbyInterface OtherActor "/Game/Blueprints/BPI_Interact.BPI_Interact_C")))
  (bind _returnvalue (UserInterface|CreateWidget "/Game/UI/Interact/W_InteractionPrompt.W_InteractionPrompt_C"))
  (bind _output_get (Variables|Default|SetWidgetInteract _returnvalue))
  (UserInterface|Viewport|AddtoViewport _output_get 0))

(event OnComponentEndOverlap(Interact)
  (params (OverlappedComponent :type Primitive%20Component%20Object%20Reference) (OtherActor :type Actor%20Object%20Reference) (OtherComp :type Primitive%20Component%20Object%20Reference) (OtherBodyIndex :type Integer))
  (Utilities|IsValid (Variables|Default|GetDialogueActor)
    (:Is%20Valid
      (bind _foundwidgets (Widget|GetAllWidgetsOfClass "/Game/UI/Interact/W_InteractionPrompt.W_InteractionPrompt_C" true))
      (for _array_element _foundwidgets
        (Widget|RemovefromParent _array_element))
      (Variables|Default|SetDialogueActor 0))))

(event Input|EnhancedActionEvents|EnhancedInputActionIA_Interact
  (params (ActionValue :type Boolean) (ElapsedSeconds :type Float%20%28double-precision%29) (TriggeredSeconds :type Float%20%28double-precision%29) (InputAction :type Input%20Action%20Object%20Reference :default "/Game/Input/Actions/IA_Interact.IA_Interact"))
  (bind _dialogueactor (Variables|Default|GetDialogueActor))
  (:Started
    (Utilities|IsValid _dialogueactor
      (:Is%20Valid
        (if (Variables|/Game/NPC/BP_BaseNPC.BP_BaseNPC_C|GetIsTalkable? (Variables|Default|GetNPC))
          (Class|BPIInteract|Interactwith(Message) _dialogueactor self (Variables|Default|GetNPC))
          (else
            (Class|BPIInteract|ComeLater(Message) _dialogueactor)))))))

(event EventBeginPlay
  (Audio|SpawnSound2D "/Game/Assets/music/Love_or_Lust_-_Quincas_Moreira.Love_or_Lust_-_Quincas_Moreira" 1.0 1.0 0.0 0)
  (bind _returnvalue (UserInterface|CreateWidget "/Game/Intro/W_IntroOne.W_IntroOne_C"))
  (bind _output_get (Variables|Default|Setintrowidget _returnvalue))
  (UserInterface|Viewport|AddtoViewport _output_get 0)
  (Variables|Default|Setintro_One true))

(event Input|KeyboardEvents|Enter
  (params (Key :type Key%20Structure :default "None"))
  (:Pressed
    (if (Variables|Default|Getintro_One)
      (bind _foundwidgets (Widget|GetAllWidgetsOfClass "/Game/Intro/W_IntroOne.W_IntroOne_C" false))
      (for _array_element _foundwidgets
        (Widget|RemovefromParent _array_element))
      (bind _returnvalue (UserInterface|CreateWidget "/Game/Intro/W_IntroOneText.W_IntroOneText_C"))
      (bind _output_get (Variables|Default|Setintrowidgettext _returnvalue))
      (UserInterface|Viewport|AddtoViewport _output_get 0)
      (Variables|Default|SetIntroTextOne true)
      (Variables|Default|Setintro_One false)
      (elif (Variables|Default|GetIntroTextOne)
        (bind _foundwidgets_2 (Widget|GetAllWidgetsOfClass "/Game/Intro/W_IntroOneText.W_IntroOneText_C" false))
        (for _array_element_2 _foundwidgets_2
          (Widget|RemovefromParent _array_element_2))
        (bind _returnvalue_2 (UserInterface|CreateWidget "/Game/tutorial/WB_Tutorial.WB_Tutorial_C"))
        (bind _output_get_2 (Variables|Default|SetNewVar _returnvalue_2))
        (UserInterface|Viewport|AddtoViewport _output_get_2 0)
        (Variables|Default|SetIntroTextOne false)
        (Variables|Default|Settuturoial true)
        (elif (Variables|Default|Gettuturoial)
          (bind _foundwidgets_3 (Widget|GetAllWidgetsOfClass "/Game/tutorial/WB_Tutorial.WB_Tutorial_C" false))
          (for _array_element_3 _foundwidgets_3
            (Widget|RemovefromParent _array_element_3))
          (Variables|Default|Settuturoial false)
          (Variables|/Game/Dialogue/BP_DialogueComponent.BP_DialogueComponent_C|SetIsInGame (Variables|Default|GetBP_DialogueComponent) true))))))

(fn ConstructionScript)