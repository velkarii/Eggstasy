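; Dialogue component that runs NPC conversations from linked DataTable rows, locking player movement while the dialogue window is open.
; Interactwith checks the NPC's required item, then opens, advances or closes dialogue, adding up to two answers on open-ended first rows.
; OptionSelected raises relationship for good options (bad ones do nothing) and shows a timed ending screen for hardcoded row "12".
; ComeLater toggles a talk-later line; leaving after open-ended dialogue makes that NPC untalkable.
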(event Custom|Option%20Selected
  (params (RowName :type Name) (DataTable :type Data%20Table%20Object%20Reference))
  (bind _returnvalue (Game|GetPlayerController 0))
  (bind _talking_npc (Variables|Default|GetTalking%20NPC))
  (bind _dialoguewidget (Variables|Default|GetDialogueWidget))
  (bind _returnvalue_2 (Utilities|GetObjectName _talking_npc))
  (bind _returnvalue_3 (Utilities|String|StringToName _returnvalue_2))
  (if (== RowName "12")
    (Input|DisableInput (Game|GetPlayerCharacter 0) (Game|GetPlayerController 0))
    (bind _returnvalue_4 (Utilities|GetDataTableRow DataTable "12")
      (:then
        (bind _returnvalue_5 (UserInterface|CreateWidget "/Game/UI/Ending/W_Ending.W_Ending_C" 0 (Utilities|Text|ToText(Name) (Variables|Default|GetName)) (.Dialogue (Utilities|Struct|BreakS_Dialogue _returnvalue_4))))
        (bind _output_get (Variables|Default|SetEndWid _returnvalue_5))
        (Appearance|SetBrushfromTexture (Variables|/Game/UI/Ending/W_Ending.W_Ending_C|GetBackground _output_get) (Variables|Default|GetEndingPicture) false)
        (UserInterface|Viewport|AddtoViewport _output_get 0)
        (Utilities|FlowControl|Delay 2e+01)
        (Input|EnableInput _returnvalue _returnvalue)
        (Widget|RemovefromParent _output_get)
        (CallFunction|LeaveDialogue)))
    (else
      (for _array_element (Variables|Default|GetGoodOptions)
        (if (== _array_element RowName)
          (bind _asbp_base_npc (Utilities|Casting|CastToBP_BaseNPC _talking_npc))
          (Default|UpdateRelationship (Variables|Default|GetDialogueWidget) (Math|Integer|Clamp(Integer) (+ (.Value (Utilities|Map|Find (Variables|/Game/NPC/BP_BaseNPC.BP_BaseNPC_C|GetRelationshipLevels _asbp_base_npc) _returnvalue_3)) 1) 0 5))
          (bind _asbp_base_npc_2 (Utilities|Casting|CastToBP_BaseNPC (Variables|Default|GetTalking%20NPC)))
          (Utilities|Map|Add (Variables|/Game/NPC/BP_BaseNPC.BP_BaseNPC_C|GetRelationshipLevels _asbp_base_npc_2) _returnvalue_3 (Math|Integer|Clamp(Integer) (+ 1 (.Value (Utilities|Map|Find (Variables|/Game/NPC/BP_BaseNPC.BP_BaseNPC_C|GetRelationshipLevels _asbp_base_npc_2) _returnvalue_3))) 0 5))
          (Variables|Default|SetRelationship%20Levels (Variables|/Game/NPC/BP_BaseNPC.BP_BaseNPC_C|GetRelationshipLevels _asbp_base_npc_2))))
      (for _array_element_2 (Variables|Default|GetBadOptions)
        (if (== _array_element_2 RowName)
          _))
      (bind _returnvalue_6 (Utilities|GetDataTableRow DataTable RowName)
        (:then
          (Widget|Panel|ClearChildren (Variables|/Game/UI/Dialogue/WB_DialogueWindow.WB_DialogueWindow_C|GetAnswerOne _dialoguewidget))
          (Default|UpdateDialogue _dialoguewidget (.Dialogue (Utilities|Struct|BreakS_Dialogue _returnvalue_6)))
          (Variables|Default|SetRow%20Name (.Row (Utilities|Struct|BreakS_Dialogue _returnvalue_6)))
          (Variables|Default|SetData%20Table (.Datatable (Utilities|Struct|BreakS_Dialogue _returnvalue_6)))
          (Variables|Default|SetEndDialogue (.EndDialogue? (Utilities|Struct|BreakS_Dialogue _returnvalue_6))))))))

(event EventLeaveDialogue
  (bind _returnvalue (Game|GetPlayerController 0))
  (Utilities|IsValid (Variables|Default|GetDialogueWidget)
    (:Is%20Valid
      (Widget|RemovefromParent (Variables|Default|GetDialogueWidget))
      (bind _returnvalue_2 (UserInterface|CreateWidget "/Game/UI/Interact/W_InteractionPrompt.W_InteractionPrompt_C"))
      (UserInterface|Viewport|AddtoViewport _returnvalue_2 0)
      (Variables|Default|SetEndDialogue false)
      (Variables|Default|SetDialogueWidget 0)
      (Input|SetInputModeGameOnly _returnvalue false)
      (Variables|/Script/Engine.PlayerController|SetbShowMouseCursor _returnvalue false)
      (Pawn|Components|CharacterMovement|SetMovementMode (Variables|/Script/Engine.Character|GetCharacterMovement (Game|GetPlayerCharacter 0)) "MOVE_Walking" 0)
      (bind _outactors (Actor|GetAllActorswithInterface "/Game/Blueprints/BPI_Interact.BPI_Interact_C"))
      (for _array_element _outactors
        (bind _asbp_base_npc (Utilities|Casting|CastToBP_BaseNPC _array_element))
        (Variables|/Game/NPC/BP_BaseNPC.BP_BaseNPC_C|SetIsTalkable? _asbp_base_npc true))
      (if (Variables|Default|GetShouldBeBlocked)
        (bind _asbp_base_npc_2 (Utilities|Casting|CastToBP_BaseNPC (Variables|Default|GetTalking%20NPC)))
        (Variables|/Game/NPC/BP_BaseNPC.BP_BaseNPC_C|SetIsTalkable? _asbp_base_npc_2 false)))))

(event EventComeLater
  (bind _returnvalue (Game|GetPlayerController 0))
  (bind _returnvalue_2 (Game|GetPlayerController 0))
  (bind _talking_npc (Variables|Default|GetTalking%20NPC))
  (bind _foundwidgets (Widget|GetAllWidgetsOfClass "/Game/UI/Interact/W_InteractionPrompt.W_InteractionPrompt_C" true))
  (for _array_element _foundwidgets
    (Widget|RemovefromParent _array_element))
  (if (Variables|Default|GetTalkLaterEnd)
    (Widget|RemovefromParent (Variables|Default|GetDialogueWidget))
    (Variables|Default|SetTalkLaterEnd false)
    (Variables|Default|SetDialogueWidget 0)
    (Input|SetInputModeGameOnly _returnvalue_2 false)
    (Variables|/Script/Engine.PlayerController|SetbShowMouseCursor _returnvalue_2 false)
    (Pawn|Components|CharacterMovement|SetMovementMode (Variables|/Script/Engine.Character|GetCharacterMovement (Game|GetPlayerCharacter 0)) "MOVE_Walking" 0)
    (bind _returnvalue_3 (UserInterface|CreateWidget "/Game/UI/Interact/W_InteractionPrompt.W_InteractionPrompt_C"))
    (UserInterface|Viewport|AddtoViewport _returnvalue_3 0)
    (else
      (bind _returnvalue_4 (Utilities|GetDataTableRow (Variables|Default|GetTalkLaterTable) (Variables|Default|GetTalkLaterRow))
        (:then
          (bind _returnvalue_5 (UserInterface|CreateWidget "/Game/UI/Dialogue/WB_DialogueWindow.WB_DialogueWindow_C" 0 (Utilities|Text|ToText(Name) (Variables|Default|GetName)) (.Dialogue (Utilities|Struct|BreakS_Dialogue _returnvalue_4)) (Variables|Default|GetWidgetImage)))
          (bind _output_get (Variables|Default|SetDialogueWidget _returnvalue_5))
          (bind _asbp_base_npc (Utilities|Casting|CastToBP_BaseNPC _talking_npc))
          (Default|UpdateRelationship _output_get (.Value (Utilities|Map|Find (Variables|/Game/NPC/BP_BaseNPC.BP_BaseNPC_C|GetRelationshipLevels _asbp_base_npc) (Utilities|String|StringToName (Utilities|GetObjectName _talking_npc)))))
          (UserInterface|Viewport|AddtoViewport _output_get 0)
          (Pawn|Components|CharacterMovement|SetMovementMode (Variables|/Script/Engine.Character|GetCharacterMovement (Game|GetPlayerCharacter 0)) "MOVE_None" 0)
          (Input|SetInputModeGameandUI _returnvalue 0 "DoNotLock" true false)
          (Variables|/Script/Engine.PlayerController|SetbShowMouseCursor _returnvalue true)
          (Variables|Default|SetTalkLaterEnd true))))))

(event EventInteractwith
  (params (Player :type BP%20Player%20Character%20Object%20Reference) (TalkingNPC :type Actor%20Object%20Reference))
  (bind _returnvalue (Game|GetPlayerController 0))
  (bind _returnvalue_2 (Game|GetPlayerController 0))
  (bind _asbp_base_npc (Utilities|Casting|CastToBP_BaseNPC TalkingNPC))
  (if (Utilities|Text|TextIsEmpty (Variables|/Game/NPC/BP_BaseNPC.BP_BaseNPC_C|GetItemId _asbp_base_npc))
    (bind _foundwidgets (Widget|GetAllWidgetsOfClass "/Game/UI/Interact/W_InteractionPrompt.W_InteractionPrompt_C" true :!label _label))
    (for _array_element _foundwidgets
      (Widget|RemovefromParent _array_element))
    (Variables|Default|SetTalking%20NPC TalkingNPC)
    (if (Variables|Default|GetEndDialogue)
      (Widget|RemovefromParent (Variables|Default|GetDialogueWidget))
      (bind _returnvalue_3 (UserInterface|CreateWidget "/Game/UI/Interact/W_InteractionPrompt.W_InteractionPrompt_C"))
      (UserInterface|Viewport|AddtoViewport _returnvalue_3 0)
      (Variables|Default|SetEndDialogue false)
      (Variables|Default|SetDialogueWidget 0)
      (Input|SetInputModeGameOnly _returnvalue_2 false)
      (Variables|/Script/Engine.PlayerController|SetbShowMouseCursor _returnvalue_2 false)
      (Pawn|Components|CharacterMovement|SetMovementMode (Variables|/Script/Engine.Character|GetCharacterMovement (Game|GetPlayerCharacter 0)) "MOVE_Walking" 0)
      (bind _outactors (Actor|GetAllActorswithInterface "/Game/Blueprints/BPI_Interact.BPI_Interact_C"))
      (for _array_element_2 _outactors
        (bind _asbp_base_npc_2 (Utilities|Casting|CastToBP_BaseNPC _array_element_2))
        (Variables|/Game/NPC/BP_BaseNPC.BP_BaseNPC_C|SetIsTalkable? _asbp_base_npc_2 true))
      (if (Variables|Default|GetShouldBeBlocked)
        (bind _asbp_base_npc_3 (Utilities|Casting|CastToBP_BaseNPC (Variables|Default|GetTalking%20NPC)))
        (Variables|/Game/NPC/BP_BaseNPC.BP_BaseNPC_C|SetIsTalkable? _asbp_base_npc_3 false))
      (else
        (Utilities|IsValid (Variables|Default|GetDialogueWidget)
          (:Is%20Valid
            (bind _returnvalue_4 (Utilities|GetDataTableRow (Variables|Default|GetData%20Table) (Variables|Default|GetRow%20Name))
              (:then
                (Default|UpdateDialogue (Variables|Default|GetDialogueWidget) (.Dialogue (Utilities|Struct|BreakS_Dialogue _returnvalue_4)))
                (Variables|Default|SetRow%20Name (.Row (Utilities|Struct|BreakS_Dialogue _returnvalue_4)))
                (Variables|Default|SetData%20Table (.Datatable (Utilities|Struct|BreakS_Dialogue _returnvalue_4)))
                (Variables|Default|SetEndDialogue (.EndDialogue? (Utilities|Struct|BreakS_Dialogue _returnvalue_4))))))
          (:Is%20Not%20Valid
            (bind _returnvalue_5 (Utilities|GetDataTableRow (Variables|Default|GetData%20Table) (Variables|Default|GetRow%20Name))
              (:then
                (bind _returnvalue_6 (UserInterface|CreateWidget "/Game/UI/Dialogue/WB_DialogueWindow.WB_DialogueWindow_C" 0 (Utilities|Text|ToText(Name) (Variables|Default|GetName)) (.Dialogue (Utilities|Struct|BreakS_Dialogue _returnvalue_5)) (Variables|Default|GetWidgetImage)))
                (bind _output_get (Variables|Default|SetDialogueWidget _returnvalue_6))
                (bind _asbp_base_npc_4 (Utilities|Casting|CastToBP_BaseNPC (Variables|Default|GetTalking%20NPC)))
                (Default|UpdateRelationship (Variables|Default|GetDialogueWidget) (.Value (Utilities|Map|Find (Variables|/Game/NPC/BP_BaseNPC.BP_BaseNPC_C|GetRelationshipLevels _asbp_base_npc_4) (Utilities|String|StringToName (Utilities|GetObjectName (Variables|Default|GetTalking%20NPC))))))
                (UserInterface|Viewport|AddtoViewport _output_get 0)
                (Variables|Default|SetRow%20Name (.Row (Utilities|Struct|BreakS_Dialogue _returnvalue_5)))
                (Variables|Default|SetData%20Table (.Datatable (Utilities|Struct|BreakS_Dialogue _returnvalue_5)))
                (Variables|Default|SetEndDialogue (.EndDialogue? (Utilities|Struct|BreakS_Dialogue _returnvalue_5)))
                (Pawn|Components|CharacterMovement|SetMovementMode (Variables|/Script/Engine.Character|GetCharacterMovement (Game|GetPlayerCharacter 0)) "MOVE_None" 0)
                (Input|SetInputModeGameandUI _returnvalue 0 "DoNotLock" true false)
                (Variables|/Script/Engine.PlayerController|SetbShowMouseCursor _returnvalue true)
                (if (.OpenEndedDialogue? (Utilities|Struct|BreakS_Dialogue _returnvalue_5))
                  (Utilities|FlowControl|Sequence
                    (:then_0
                      (bind _returnvalue_7 (UserInterface|CreateWidget "/Game/UI/Dialogue/WB_Options.WB_Options_C" 0 (Utilities|Text|ToText(Name) (.OptionName (Utilities|Struct|BreakS_DialogueOptions (Utilities|Array|Get(acopy) (.OpenEndedDialogueOptions (Utilities|Struct|BreakS_Dialogue _returnvalue_5)))))) self (.Row (Utilities|Struct|BreakS_DialogueOptions (Utilities|Array|Get(acopy) (.OpenEndedDialogueOptions (Utilities|Struct|BreakS_Dialogue _returnvalue_5))))) (.Datatable (Utilities|Struct|BreakS_DialogueOptions (Utilities|Array|Get(acopy) (.OpenEndedDialogueOptions (Utilities|Struct|BreakS_Dialogue _returnvalue_5)))))))
                      (Widget|Panel|AddChild (Variables|/Game/UI/Dialogue/WB_DialogueWindow.WB_DialogueWindow_C|GetAnswerOne (Variables|Default|GetDialogueWidget)) _returnvalue_7))
                    (:then_1
                      (Utilities|IsValid (.Datatable (Utilities|Struct|BreakS_DialogueOptions (Utilities|Array|Get(acopy) (.OpenEndedDialogueOptions (Utilities|Struct|BreakS_Dialogue _returnvalue_5)) 1)))
                        (:Is%20Valid
                          (bind _returnvalue_8 (UserInterface|CreateWidget "/Game/UI/Dialogue/WB_Options.WB_Options_C" 0 (Utilities|Text|ToText(Name) (.OptionName (Utilities|Struct|BreakS_DialogueOptions (Utilities|Array|Get(acopy) (.OpenEndedDialogueOptions (Utilities|Struct|BreakS_Dialogue _returnvalue_5)) 1)))) self (.Row (Utilities|Struct|BreakS_DialogueOptions (Utilities|Array|Get(acopy) (.OpenEndedDialogueOptions (Utilities|Struct|BreakS_Dialogue _returnvalue_5)) 1))) (.Datatable (Utilities|Struct|BreakS_DialogueOptions (Utilities|Array|Get(acopy) (.OpenEndedDialogueOptions (Utilities|Struct|BreakS_Dialogue _returnvalue_5)) 1)))))
                          (Widget|Panel|AddChild (Variables|/Game/UI/Dialogue/WB_DialogueWindow.WB_DialogueWindow_C|GetAnswerTwo (Variables|Default|GetDialogueWidget)) _returnvalue_8))))
                    (:then_2
                      (Variables|Default|SetShouldBeBlocked true)))
                  (else
                    (Variables|Default|SetShouldBeBlocked false)))))))))
    (elif (Class|InventoryComponent|HasItem (Variables|/Game/Player/BP_PlayerCharacter.BP_PlayerCharacter_C|GetInventory Player) (Utilities|String|ToString(Text) (Variables|/Game/NPC/BP_BaseNPC.BP_BaseNPC_C|GetItemId _asbp_base_npc)))
      (goto _label)
      (else
        (bind _returnvalue_9 (UserInterface|CreateWidget "/Game/Quest/Notification.Notification_C"))
        (UserInterface|Viewport|AddtoViewport _returnvalue_9 0)
        (Default|ShowMessage _returnvalue_9 (Utilities|Text|FormatText "You need to find {item} first" (Variables|/Game/NPC/BP_BaseNPC.BP_BaseNPC_C|GetItemId _asbp_base_npc)))))))